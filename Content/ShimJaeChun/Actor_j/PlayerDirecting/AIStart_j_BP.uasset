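; Trigger-box actor for player directing that hands the player character to an AI-driven move when it walks in.
; BeginPlay caches the player as AnimTestCharacter_j_BP, and the box overlap reacts only to that character when ActorToMove is valid.
; It plays the CineCamera sequence, or failing that switches the view target to CameraActor if valid.
; It then calls BeginStartAI on the character with ActorToMove.
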(event OnComponentBeginOverlap(Box)
  (params (OverlappedComponent :type Primitive%20Component%20Object%20Reference) (OtherActor :type Actor%20Object%20Reference) (OtherComp :type Primitive%20Component%20Object%20Reference) (OtherBodyIndex :type Integer) (bFromSweep :type Boolean) (SweepResult :type Hit%20Result%20Structure%20%28by%20ref%29))
  (bind _cameraactor (Variables|Default|GetCameraActor))
  (if (== OtherActor (Variables|Default|GetMyCharacter))
    (if (Utilities|IsValid (Variables|Default|GetActorToMove))
      (if (Utilities|IsValid (Variables|Default|GetCineCamera))
        (Sequencer|Player|Play (Variables|/Script/LevelSequence.LevelSequenceActor|GetSequencePlayer (Variables|Default|GetCineCamera)) :!class /Script/MovieScene.MovieSceneSequencePlayer)
        (elif (Utilities|IsValid _cameraactor)
          (Game|Player|SetViewTargetwithBlend (Game|GetPlayerController 0) _cameraactor 0.0 "VTBlend_Linear" 0.0 false)))
      (Default|BeginStartAI (Variables|Default|GetMyCharacter) (Variables|Default|GetActorToMove)))))

(event EventTick
  (params (DeltaSeconds :type Float%20%28single-precision%29)))

(event EventBeginPlay
  (bind _asanim_test_character_j_bp (Utilities|Casting|CastToAnimTestCharacter_j_BP (Game|GetPlayerCharacter 0)))
  (Variables|Default|SetMyCharacter _asanim_test_character_j_bp))

(fn ConstructionScript)