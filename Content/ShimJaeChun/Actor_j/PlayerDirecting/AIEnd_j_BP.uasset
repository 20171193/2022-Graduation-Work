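; AIEnd_j_BP is a trigger-box actor that calls EndStartAI on the player character, apparently to end an AI-directed player sequence.
; BeginPlay caches player 0 as AnimTestCharacter_j_BP, and the Box overlap responds only to that character.
; It passes its HasCamera variable to the call through a DoOnce that resets right afterward, so every new overlap can fire again.
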(event OnComponentBeginOverlap(Box)
  (params (OverlappedComponent :type Primitive%20Component%20Object%20Reference) (OtherActor :type Actor%20Object%20Reference) (OtherComp :type Primitive%20Component%20Object%20Reference) (OtherBodyIndex :type Integer) (bFromSweep :type Boolean) (SweepResult :type Hit%20Result%20Structure%20%28by%20ref%29))
  (if (== OtherActor (Variables|Default|GetMyCharacter))
    (Utilities|FlowControl|DoOnce false :!label _label
      (:Completed
        (Default|EndStartAI (Variables|Default|GetMyCharacter) (Variables|Default|GetHasCamera))
        (goto _label Reset)))))

(event Collision|EventActorBeginOverlap
  (params (OtherActor :type Actor%20Object%20Reference)))

(event EventTick
  (params (DeltaSeconds :type Float%20%28single-precision%29)))

(event EventBeginPlay
  (bind _asanim_test_character_j_bp (Utilities|Casting|CastToAnimTestCharacter_j_BP (Game|GetPlayerCharacter 0)))
  (Variables|Default|SetMyCharacter _asanim_test_character_j_bp))

(fn ConstructionScript)