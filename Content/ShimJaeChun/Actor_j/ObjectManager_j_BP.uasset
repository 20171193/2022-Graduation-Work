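; ObjectManager_j_BP is a manager actor that shows and hides a group of actors held in VisibleArrayActor.
; VisibleOn loops over the array, unhiding each actor and enabling its collision.
; VisibleOff hides each actor but disables collision on the manager itself, leaving the listed actors' collision untouched.
; Both events run only when index 0 is valid and are not called within this graph.
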(event Custom|VisibleOn
  (if (Utilities|Array|IsValidIndex (Variables|Default|GetVisibleArray_Actor))
    (for _array_element (Variables|Default|GetVisibleArray_Actor)
      (Rendering|SetActorHiddenInGame _array_element false)
      (Collision|SetActorEnableCollision _array_element true))))

(event Custom|VisibleOff
  (if (Utilities|Array|IsValidIndex (Variables|Default|GetVisibleArray_Actor))
    (for _array_element (Variables|Default|GetVisibleArray_Actor)
      (Rendering|SetActorHiddenInGame _array_element true)
      (Collision|SetActorEnableCollision false))))

(event EventBeginPlay)

(event Collision|EventActorBeginOverlap
  (params (OtherActor :type Actor%20Object%20Reference)))

(event EventTick
  (params (DeltaSeconds :type Float%20%28single-precision%29)))

(fn ConstructionScript)