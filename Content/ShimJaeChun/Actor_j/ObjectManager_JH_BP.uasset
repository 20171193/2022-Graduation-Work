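; ObjectManager_JH_BP is a manager actor that shows or hides a group of static mesh actors held in its VisibleArrayStaticmesh array.
; VisibleOn loops over the array, making each mesh component visible and enabling query and physics collision.
; VisibleOff does the reverse, hiding each mesh and disabling its collision, so hidden objects do not block anything.
; Nothing in this Blueprint calls either event, and BeginPlay, Tick and the construction script are empty.
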(event Custom|VisibleOn
  (if (Utilities|Array|IsValidIndex (Variables|Default|GetVisibleArray_Staticmesh))
    (for _array_element (Variables|Default|GetVisibleArray_Staticmesh)
      (Rendering|SetVisibility (Variables|/Script/Engine.StaticMeshActor|GetStaticMeshComponent _array_element) true false)
      (Collision|SetCollisionEnabled (Variables|/Script/Engine.StaticMeshActor|GetStaticMeshComponent _array_element) "QueryAndPhysics"))))

(event Custom|VisibleOff
  (if (Utilities|Array|IsValidIndex (Variables|Default|GetVisibleArray_Staticmesh))
    (for _array_element (Variables|Default|GetVisibleArray_Staticmesh)
      (Rendering|SetVisibility (Variables|/Script/Engine.StaticMeshActor|GetStaticMeshComponent _array_element) false false)
      (Collision|SetCollisionEnabled (Variables|/Script/Engine.StaticMeshActor|GetStaticMeshComponent _array_element) "NoCollision"))))

(event EventBeginPlay)

(event Collision|EventActorBeginOverlap
  (params (OtherActor :type Actor%20Object%20Reference)))

(event EventTick
  (params (DeltaSeconds :type Float%20%28single-precision%29)))

(fn ConstructionScript)