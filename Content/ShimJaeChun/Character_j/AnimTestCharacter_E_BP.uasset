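; Euncheol's test character Blueprint, with ladder climbing and switchable camera views.
; On BeginPlay it applies a quarter view; W, A, S and D switch between top, side, back and quarter presets, resetting actor and control rotation.
; When climbable, F enters Flying and snaps to a nearby Ledder_j_BP by its yaw, or, if already on a ladder, steps back and falls.
; An unconnected roll-montage graph never runs.
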(event Collision|EventActorBeginOverlap
  (params (OtherActor :type Actor%20Object%20Reference)))

(event EventBeginPlay
  (Development|PrintText "EuncheolCharacterMode")
  ;[1 1 1] 플레이어 시작 세팅 - 쿼터뷰
  (Variables|Default|SetcurrentMoveMode 0)
  (Transformation|SetRelativeLocationAndRotation (Variables|Default|GetCameraComponent) "-535.000000,7.500000,1135.000000" "-50.000000,0.000000,0.000000" false false)
  (bind _asanim_test_character_j_bp (Utilities|Casting|CastToAnimTestCharacter_j_BP (Game|GetPlayerCharacter 0)))
  (Transformation|SetActorRelativeRotation _asanim_test_character_j_bp "0,-50.000000,0.000000")
  (Pawn|SetControlRotation (Game|GetPlayerController 0) (Math|Rotator|MakeRotator 0.0 0.0 -5e+01)))

(event Input|ActionEvents|InputActionActRoll
  (params (Key :type Key%20Structure :default "None")))

(event Input|KeyboardEvents|F
  (params (Key :type Key%20Structure :default "None"))
  (bind _returnvalue (Game|GetPlayerCharacter 0))
  ;[1 1 1] 사다리 타기
  (:Pressed
    (if (Variables|Default|Getclimbable)
      (if (Variables|Default|GetisLadder)
        (Utilities|FlowControl|Sequence
          (:then_0
            (goto _label Reset))
          (:then_1
            ;[1 1 1] 사다리 추락
            (Transformation|SetActorRelativeLocation (+ (Transformation|GetActorLocation _returnvalue) (* (Transformation|GetActorForwardVector _returnvalue) -5e+01)))
            (Pawn|Components|CharacterMovement|SetMovementMode (Variables|Character|GetCharacterMovement) "MOVE_Falling" 0)))
        (else
          (Pawn|Components|CharacterMovement|SetMovementMode (Variables|Character|GetCharacterMovement) "MOVE_Flying" 0)
          (Variables|Default|SetisLadder true)
          (Utilities|FlowControl|Sequence
            (:then_0
              (Utilities|FlowControl|DoOnce false :!label _label
                (:Completed
                  (bind _outactors (Actor|GetAllActorsOfClass "/Game/ShimJaeChun/Actor_j/Ledder_j_BP.Ledder_j_BP_C"))
                  (bind (_array_element _array_index) (Utilities|Array|ForEachLoopwithBreak _outactors :!label _label_2)
                    (:LoopBody
                      (bind _asanim_test_character_j_bp (Utilities|Casting|CastToAnimTestCharacter_j_BP (Game|GetPlayerCharacter 0)))
                      (if (<= (Transformation|GetDistanceTo _array_element) 1.8e+02)
                        (Utilities|FlowControl|Sequence
                          (:then_0
                            (Variables|Default|SetLadder%20Index _array_index)
                            (Utilities|FlowControl|Delay 0.1)
                            (Transformation|SetActorRotation (Math|Rotator|MakeRotator (.roll (Transformation|GetActorRotation _asanim_test_character_j_bp)) (.pitch (Transformation|GetActorRotation _asanim_test_character_j_bp)) (+ (.yaw (Transformation|GetActorRotation (Variables|Default|GetLadder%20BP%20ref))) -9e+01)))
                            (Variables|Default|SetPlayer%20Z%20Location (.z (Transformation|GetActorLocation _asanim_test_character_j_bp)))
                            (if (and (<= (.yaw (Transformation|GetActorRotation (Variables|Default|GetLadder%20BP%20ref))) 185.0) (> (.yaw (Transformation|GetActorRotation (Variables|Default|GetLadder%20BP%20ref))) 175.0))
                              ;[1 1 1] -> 사다리
                              (Development|PrintString "->")
                              (Transformation|SetActorLocation (Math|Vector|MakeVector (.x (Transformation|GetActorLocation (Variables|Default|GetLadder%20BP%20ref))) (+ (.y (Transformation|GetActorLocation (Variables|Default|GetLadder%20BP%20ref))) 4e+01) (.z (Transformation|GetActorLocation _asanim_test_character_j_bp))) false false)
                              (else
                                ;[1 1 1] ^ 사다리
                                (if (and (<= (.yaw (Transformation|GetActorRotation (Variables|Default|GetLadder%20BP%20ref))) 95.0) (> (.yaw (Transformation|GetActorRotation (Variables|Default|GetLadder%20BP%20ref))) 85.0))
                                  (Development|PrintString "^")
                                  (Transformation|SetActorLocation (Math|Vector|MakeVector (- (.x (Transformation|GetActorLocation (Variables|Default|GetLadder%20BP%20ref))) 4e+01) (.y (Transformation|GetActorLocation (Variables|Default|GetLadder%20BP%20ref))) (Variables|Default|GetPlayer%20Z%20Location)) false false)
                                  (else
                                    ;[1 1 1] V 사다리
                                    (if (and (<= (.yaw (Transformation|GetActorRotation (Variables|Default|GetLadder%20BP%20ref))) 275.0) (> (.yaw (Transformation|GetActorRotation (Variables|Default|GetLadder%20BP%20ref))) 265.0))
                                      (Development|PrintString "V")
                                      (Transformation|SetActorLocation (Math|Vector|MakeVector (+ (.x (Transformation|GetActorLocation (Variables|Default|GetLadder%20BP%20ref))) 4e+01) (.y (Transformation|GetActorLocation (Variables|Default|GetLadder%20BP%20ref))) (Variables|Default|GetPlayer%20Z%20Location)) false false)
                                      (else
                                        ;[1 1 1] <- 사다리
                                        (if (and (<= (.yaw (Transformation|GetActorRotation (Variables|Default|GetLadder%20BP%20ref))) 5.0) (> (.yaw (Transformation|GetActorRotation (Variables|Default|GetLadder%20BP%20ref))) -5.0))
                                          (Development|PrintString "<-")
                                          (Transformation|SetActorLocation (Math|Vector|MakeVector (.x (Transformation|GetActorLocation (Variables|Default|GetLadder%20BP%20ref))) (+ (.y (Transformation|GetActorLocation (Variables|Default|GetLadder%20BP%20ref))) 4e+01) (Variables|Default|GetPlayer%20Z%20Location)) false false)))))))))
                          (:then_1
                            (goto _label_2 Break))
                          (:then_2
                            (Variables|Default|SetLadder%20BP%20ref (Utilities|Array|Get(acopy) _outactors (Variables|Default|GetLadder%20Index)))))))))))))))))

(event Input|KeyboardEvents|A
  (params (Key :type Key%20Structure :default "None"))
  ;[1 1 1] 사이드 뷰모드 세팅
  (:Pressed
    (Variables|Default|SetcurrentMoveMode 0)
    (Transformation|SetRelativeLocationAndRotation (Variables|Default|GetCameraComponent) "0.000000,-600.000000,100.000000" "0.000000,90.000000,0.000000" false false)
    (bind _asanim_test_character_j_bp (Utilities|Casting|CastToAnimTestCharacter_j_BP (Game|GetPlayerCharacter 0)))
    (Transformation|SetActorRelativeRotation _asanim_test_character_j_bp)
    (Pawn|SetControlRotation (Game|GetPlayerController 0) (Math|Rotator|MakeRotator 0.0 0.0 0.0))))

(event Input|KeyboardEvents|W
  (params (Key :type Key%20Structure :default "None"))
  ;[1 1 1] 탑 뷰모드 세팅
  (:Pressed
    (Variables|Default|SetcurrentMoveMode 0)
    (Transformation|SetRelativeLocationAndRotation (Variables|Default|GetCameraComponent) "300.000000,0.000000,1000.000000" "-90.000000,0.000000,0.000000" false false)
    (bind _asanim_test_character_j_bp (Utilities|Casting|CastToAnimTestCharacter_j_BP (Game|GetPlayerCharacter 0)))
    (Transformation|SetActorRelativeRotation _asanim_test_character_j_bp)
    (Pawn|SetControlRotation (Game|GetPlayerController 0) (Math|Rotator|MakeRotator 0.0 0.0 0.0))))

(event Input|KeyboardEvents|D
  (params (Key :type Key%20Structure :default "None"))
  ;[1 1 1] 쿼터 뷰모드 세팅
  (:Pressed
    (Variables|Default|SetcurrentMoveMode 0)
    (Transformation|SetRelativeLocationAndRotation (Variables|Default|GetCameraComponent) "-535.000000,7.500000,1135.000000" "-50.000000,0.000000,0.000000" false false)
    (bind _asanim_test_character_j_bp (Utilities|Casting|CastToAnimTestCharacter_j_BP (Game|GetPlayerCharacter 0)))
    (Transformation|SetActorRelativeRotation _asanim_test_character_j_bp "0,-50.000000,0.000000")
    (Pawn|SetControlRotation (Game|GetPlayerController 0) (Math|Rotator|MakeRotator 0.0 0.0 -5e+01))))

(event Input|KeyboardEvents|S
  (params (Key :type Key%20Structure :default "None"))
  ;[1 1 1] 백 뷰모드 세팅
  (:Pressed
    (Variables|Default|SetcurrentMoveMode 0)
    (Transformation|SetRelativeLocationAndRotation (Variables|Default|GetCameraComponent) "-1620.000000,0.000000,80.000000" "0, 0, 0" false false)
    (bind _asanim_test_character_j_bp (Utilities|Casting|CastToAnimTestCharacter_j_BP (Game|GetPlayerCharacter 0)))
    (Transformation|SetActorRelativeRotation _asanim_test_character_j_bp)
    (Pawn|SetControlRotation (Game|GetPlayerController 0) (Math|Rotator|MakeRotator 0.0 0.0 0.0))))

(fn ConstructionScript)