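; Player character that switches between top, side, back and quarter views with W/A/S/D, repositioning the camera and resetting rotation.
; ChangeViewCheck capsule-traces for side and back views, rejecting blocked switches and toggling visibility and collision of "Wall"-tagged components.
; Damage triggers knockback by causer yaw, invincibility with swapped materials and ortho-width zoom shake; death resets to origin.
; F handles ladder snapping and release; Roll changes speed and capsule height, with timer cooldown.
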(event Custom|HitEffect
  ;[1 1 1] Hit 관련 이벤트
  (Variables|Default|SetbCanBeDamaged false)
  (Rendering|Material|SetMaterial (Variables|Character|GetMesh) 0 "/Game/ShimJaeChun/Archer_j/Mats/Akai_MAT_Damage_inst_j.Akai_MAT_Damage_inst_j")
  (Rendering|Material|SetMaterial (Variables|Character|GetMesh) 3 "/Game/ShimJaeChun/Archer_j/Mats/Body_MAT_Inst_j.Body_MAT_Inst_j")
  (Utilities|FlowControl|Delay (Variables|Default|GetinvincibleTime))
  (Rendering|Material|SetMaterial (Variables|Character|GetMesh) 0 "/Game/ShimJaeChun/Archer_j/Mats/Akai_MAT_Damage_j.Akai_MAT_Damage_j")
  (Rendering|Material|SetMaterial (Variables|Character|GetMesh) 3 "/Game/ShimJaeChun/Archer_j/Mats/Body_MAT.Body_MAT")
  (Variables|Default|SetbCanBeDamaged true))

(event Collision|EventActorBeginOverlap
  (params (OtherActor :type Actor%20Object%20Reference)))

(event EventBeginPlay
  ;[1 1 1] 플레이어 시작 세팅 - 쿼터뷰
  (Variables|Default|SetcurrentMoveMode "QuarterViewMode")
  (Transformation|SetRelativeLocationAndRotation (Variables|Default|GetCameraComponent) "-535.000000,7.500000,1135.000000" "-50.000000,0.000000,0.000000" false false)
  (bind _asanim_test_character_j_bp (Utilities|Casting|CastToAnimTestCharacter_j_BP (Game|GetPlayerCharacter 0)))
  (Transformation|SetActorRelativeRotation _asanim_test_character_j_bp "0,-50.000000,0.000000")
  (Pawn|SetControlRotation (Game|GetPlayerController 0) (Math|Rotator|MakeRotator 0.0 0.0 -5e+01)))

(event Game|Damage|EventAnyDamage
  (params (Damage :type Float%20%28single-precision%29) (DamageType :type Damage%20Type%20Object%20Reference) (InstigatedBy :type Controller%20Object%20Reference) (DamageCauser :type Actor%20Object%20Reference))
  (bind _returnvalue (Game|GetPlayerController 0))
  ;[1 1 1] 데미지처리
  (bind _output_get (Variables|Default|SetplayerHp (- (Variables|Default|GetplayerHp) (Math|Float|Truncate Damage))))
  (if (<= _output_get 0)
    ;[1 1 1] Death처리
    (bind _returnvalue_2 (Animation|PlayAnimMontage "/Game/ShimJaeChun/Anim_j/StandingDeath_AMG_j.StandingDeath_AMG_j" 1.0 "None"))
    (Input|DisableInput _returnvalue)
    (Utilities|FlowControl|Delay _returnvalue_2)
    (Transformation|SetActorLocation "0, 0, 0" false false)
    (Input|EnableInput _returnvalue)
    (Variables|Default|SetplayerHp 5)
    (else
      ;[1 1 1] 피격 처리
      (if (Utilities|IsValid DamageCauser)
        (Variables|Default|SetdamageActorRotZ (.yaw (Transformation|GetActorRotation DamageCauser)))
        (if (and (<= (Variables|Default|GetdamageActorRotZ) 1e+01) (> (Variables|Default|GetdamageActorRotZ) -1e+01))
          (Development|PrintString "0도")
          (Character|LaunchCharacter self (Math|Vector|MakeVector 0.0 1e+03 5e+01) true false)
          (Animation|PlayAnimMontage "/Game/ShimJaeChun/Anim_j/HitReaction_AM.HitReaction_AM" 1.0 "None" :!label _label)
          (CallFunction|HitEffect)
          (bind _zoom (Timeline|CameraShakeTimeline Play)
            (:Update
              (Class|CameraComponent|SetOrthoWidth (Variables|Default|GetCameraComponent) _zoom))
            (:Finished
              (if true
                (Timeline|CameraShakeTimeline SetNewTime))))
          (elif (or (and (<= (Variables|Default|GetdamageActorRotZ) 1e+02) (> (Variables|Default|GetdamageActorRotZ) 8e+01)) (and (<= (Variables|Default|GetdamageActorRotZ) -2.6e+02) (> (Variables|Default|GetdamageActorRotZ) -2.8e+02)))
            (Development|PrintString "90, -270도")
            (Character|LaunchCharacter self (Math|Vector|MakeVector -1e+03 0.0 5e+01) true true)
            (goto _label)
            (elif (or (and (<= (Variables|Default|GetdamageActorRotZ) 1.9e+02) (> (Variables|Default|GetdamageActorRotZ) 1.7e+02)) (and (<= (Variables|Default|GetdamageActorRotZ) -1.7e+02) (> (Variables|Default|GetdamageActorRotZ) -1.9e+02)))
              (Development|PrintString "180, -180도")
              (Character|LaunchCharacter self (Math|Vector|MakeVector 0.0 -1e+03 5e+01) true false)
              (goto _label)
              (elif (or (and (<= (Variables|Default|GetdamageActorRotZ) 2.8e+02) (> (Variables|Default|GetdamageActorRotZ) 2.6e+02)) (and (<= (Variables|Default|GetdamageActorRotZ) -8e+01) (> (Variables|Default|GetdamageActorRotZ) -1e+02)))
                (Development|PrintString "270, -90도")
                (Character|LaunchCharacter self (Math|Vector|MakeVector 1e+03 0.0 5e+01) true false)
                (goto _label)))))))))

(event Input|ActionEvents|InputActionRoll
  (params (Key :type Key%20Structure :default "None"))
  (bind _charactermovement (Variables|Character|GetCharacterMovement))
  (bind _charactermovement_2 (Variables|Character|GetCharacterMovement))
  ;[1 1 1] 구르기
  (:Pressed
    (if (Variables|Default|GetrollAble)
      (if (Variables|Default|GetrollCooltime)
        (Development|PrintString "Not yet Roll" :!label _label)
        (else
          (Variables|Default|SetrollCooltime true)
          (bind _returnvalue (Utilities|Time|SetTimerbyFunctionName self "Roll Cool Down" 0.1 true))
          (Variables|Default|SetrcdTH _returnvalue)
          (if (Variables|Default|GetbIsCrouched)
            (Variables|/Script/Engine.CharacterMovementComponent|SetMaxWalkSpeedCrouched (Variables|Character|GetCharacterMovement) 8e+02)
            (else
              (Pawn|Components|CharacterMovement|SetMovementMode _charactermovement_2 "MOVE_Flying" 0)
              (Variables|/Script/Engine.CharacterMovementComponent|SetMaxFlySpeed _charactermovement_2 8e+02)
              (Components|Capsule|SetCapsuleHalfHeight (Variables|Default|GetCapsuleComponent) 4e+01 true)))
          (bind _returnvalue_2 (Animation|PlayAnimMontage "/Game/ShimJaeChun/Anim_j/Rolling_AMG_j.Rolling_AMG_j" 1.5 "None"))
          (Utilities|FlowControl|Delay (- _returnvalue_2 0.5))
          (if (Variables|Default|GetbIsCrouched)
            (Variables|/Script/Engine.CharacterMovementComponent|SetMaxWalkSpeedCrouched (Variables|Character|GetCharacterMovement) 1.5e+02)
            (else
              (Components|Capsule|SetCapsuleHalfHeight (Variables|Default|GetCapsuleComponent) 88.0 true)
              (Pawn|Components|CharacterMovement|SetMovementMode _charactermovement "MOVE_Walking" 0)
              (Variables|/Script/Engine.CharacterMovementComponent|SetMaxFlySpeed _charactermovement 6e+02)))))
      (else
        (goto _label)))))

(event Input|KeyboardEvents|F
  (params (Key :type Key%20Structure :default "None"))
  (bind _returnvalue (Game|GetPlayerCharacter 0))
  ;[1 1 1] 사다리 타기
  (:Pressed
    (if (Variables|Default|Getclimbable2)
      (if (Variables|Default|GetIsLadder2)
        (Utilities|FlowControl|Sequence
          (:then_0
            (goto _label Reset))
          (:then_1
            ;[1 1 1] 사다리 추락
            (Transformation|SetActorRelativeLocation (+ (Transformation|GetActorLocation _returnvalue) (* (Transformation|GetActorForwardVector _returnvalue) -5e+01)))
            (Pawn|Components|CharacterMovement|SetMovementMode (Variables|Character|GetCharacterMovement) "MOVE_Falling" 0)))
        (else
          (Pawn|Components|CharacterMovement|SetMovementMode (Variables|Character|GetCharacterMovement) "MOVE_Flying" 0)
          (Variables|Default|SetIsLadder2 true)
          (Utilities|FlowControl|Sequence
            (:then_0
              (Utilities|FlowControl|DoOnce false :!label _label
                (:Completed
                  (bind _outactors (Actor|GetAllActorsOfClass "/Game/ShimJaeChun/Actor_j/Ledder_j_BP.Ledder_j_BP_C"))
                  (bind (_array_element _array_index) (Utilities|Array|ForEachLoopwithBreak _outactors :!label _label_2)
                    (:LoopBody
                      (bind _asanim_test_character_j_bp (Utilities|Casting|CastToAnimTestCharacter_j_BP (Game|GetPlayerCharacter 0)))
                      (if (<= (Transformation|GetDistanceTo _array_element) 1.8e+02)
                        (Utilities|FlowControl|Sequence
                          (:then_0
                            (Variables|Default|SetLadder%20Index _array_index)
                            (Utilities|FlowControl|Delay 0.1)
                            (Transformation|SetActorRotation (Math|Rotator|MakeRotator (.roll (Transformation|GetActorRotation _asanim_test_character_j_bp)) (.pitch (Transformation|GetActorRotation _asanim_test_character_j_bp)) (+ (.yaw (Transformation|GetActorRotation (Variables|Default|GetLadder%20BP%20ref))) -9e+01)))
                            ;[1 1 1] -> 사다리
                            (Variables|Default|SetPlayer%20Z%20Location (.z (Transformation|GetActorLocation _asanim_test_character_j_bp)))
                            (if (and (<= (.yaw (Transformation|GetActorRotation (Variables|Default|GetLadder%20BP%20ref))) 185.0) (> (.yaw (Transformation|GetActorRotation (Variables|Default|GetLadder%20BP%20ref))) 175.0))
                              (Development|PrintString "->")
                              (Transformation|SetActorLocation (Math|Vector|MakeVector (.x (Transformation|GetActorLocation (Variables|Default|GetLadder%20BP%20ref))) (+ (.y (Transformation|GetActorLocation (Variables|Default|GetLadder%20BP%20ref))) 4e+01) (.z (Transformation|GetActorLocation _asanim_test_character_j_bp))) false false)
                              (else
                                ;[1 1 1] ^ 사다리
                                (if (and (<= (.yaw (Transformation|GetActorRotation (Variables|Default|GetLadder%20BP%20ref))) 95.0) (> (.yaw (Transformation|GetActorRotation (Variables|Default|GetLadder%20BP%20ref))) 85.0))
                                  (Development|PrintString "^")
                                  (Transformation|SetActorLocation (Math|Vector|MakeVector (- (.x (Transformation|GetActorLocation (Variables|Default|GetLadder%20BP%20ref))) 4e+01) (.y (Transformation|GetActorLocation (Variables|Default|GetLadder%20BP%20ref))) (Variables|Default|GetPlayer%20Z%20Location)) false false)
                                  (else
                                    ;[1 1 1] V 사다리
                                    (if (and (<= (.yaw (Transformation|GetActorRotation (Variables|Default|GetLadder%20BP%20ref))) 275.0) (> (.yaw (Transformation|GetActorRotation (Variables|Default|GetLadder%20BP%20ref))) 265.0))
                                      (Development|PrintString "V")
                                      (Transformation|SetActorLocation (Math|Vector|MakeVector (+ (.x (Transformation|GetActorLocation (Variables|Default|GetLadder%20BP%20ref))) 4e+01) (.y (Transformation|GetActorLocation (Variables|Default|GetLadder%20BP%20ref))) (Variables|Default|GetPlayer%20Z%20Location)) false false)
                                      (else
                                        ;[1 1 1] <- 사다리
                                        (if (and (<= (.yaw (Transformation|GetActorRotation (Variables|Default|GetLadder%20BP%20ref))) 5.0) (> (.yaw (Transformation|GetActorRotation (Variables|Default|GetLadder%20BP%20ref))) -5.0))
                                          (Development|PrintString "<-")
                                          (Transformation|SetActorLocation (Math|Vector|MakeVector (.x (Transformation|GetActorLocation (Variables|Default|GetLadder%20BP%20ref))) (+ (.y (Transformation|GetActorLocation (Variables|Default|GetLadder%20BP%20ref))) 4e+01) (Variables|Default|GetPlayer%20Z%20Location)) false false)))))))))
                          (:then_1
                            (goto _label_2 Break))
                          (:then_2
                            (Variables|Default|SetLadder%20BP%20ref (Utilities|Array|Get(acopy) _outactors (Variables|Default|GetLadder%20Index)))))))))))))))))

(event Input|KeyboardEvents|A
  (params (Key :type Key%20Structure :default "None"))
  ;[1 1 1] 사이드 뷰모드 세팅
  (:Pressed
    (if (Utilities|Enum|NotEqual(Enum) (Variables|Default|GetcurrentMoveMode) "SideViewMode")
      (bind _checkresult (CallFunction|ChangeViewCheck "SideViewMode"))
      (if _checkresult
        (Variables|Default|SetcurrentMoveMode "SideViewMode")
        (Class|CameraComponent|SetOrthoWidth (Variables|Default|GetCameraComponent) 2e+03)
        (Transformation|SetRelativeLocationAndRotation (Variables|Default|GetCameraComponent) "280.000000,-100.000000,320.000000" "0.000000,90.000000,0.000000" false false)
        (bind _asanim_test_character_j_bp (Utilities|Casting|CastToAnimTestCharacter_j_BP (Game|GetPlayerCharacter 0)))
        (Transformation|SetActorRelativeRotation _asanim_test_character_j_bp)
        (Pawn|SetControlRotation (Game|GetPlayerController 0) (Math|Rotator|MakeRotator 0.0 0.0 0.0))))))

(event Input|KeyboardEvents|W
  (params (Key :type Key%20Structure :default "None"))
  ;[1 1 1] 탑 뷰모드 세팅
  (:Pressed
    (if (Utilities|Enum|NotEqual(Enum) (Variables|Default|GetcurrentMoveMode) "TopViewMode")
      (bind _checkresult (CallFunction|ChangeViewCheck "TopViewMode"))
      (if _checkresult
        (Variables|Default|SetcurrentMoveMode "TopViewMode")
        (Transformation|SetRelativeLocationAndRotation (Variables|Default|GetCameraComponent) "300.000000,0.000000,1000.000000" "-90.000000,0.000000,0.000000" false false)
        (bind _asanim_test_character_j_bp (Utilities|Casting|CastToAnimTestCharacter_j_BP (Game|GetPlayerCharacter 0)))
        (Transformation|SetActorRelativeRotation _asanim_test_character_j_bp)
        (Pawn|SetControlRotation (Game|GetPlayerController 0) (Math|Rotator|MakeRotator 0.0 0.0 0.0))))))

(event Input|KeyboardEvents|D
  (params (Key :type Key%20Structure :default "None"))
  ;[1 1 1] 쿼터 뷰모드 세팅
  (:Pressed
    (if (Utilities|Enum|NotEqual(Enum) (Variables|Default|GetcurrentMoveMode) "QuarterViewMode")
      (bind _checkresult (CallFunction|ChangeViewCheck "QuarterViewMode"))
      (if _checkresult
        (Variables|Default|SetcurrentMoveMode "QuarterViewMode")
        (Class|CameraComponent|SetOrthoWidth (Variables|Default|GetCameraComponent) 3e+03)
        (Transformation|SetRelativeLocationAndRotation (Variables|Default|GetCameraComponent) "-535.000000,7.500000,1135.000000" "-50.000000,0.000000,0.000000" false false)
        (bind _asanim_test_character_j_bp (Utilities|Casting|CastToAnimTestCharacter_j_BP (Game|GetPlayerCharacter 0)))
        (Transformation|SetActorRelativeRotation _asanim_test_character_j_bp "0,-50.000000, 0")
        (Pawn|SetControlRotation (Game|GetPlayerController 0) (Math|Rotator|MakeRotator 0.0 0.0 -5e+01))))))

(event Input|KeyboardEvents|S
  (params (Key :type Key%20Structure :default "None"))
  ;[1 1 1] 백 뷰모드 세팅
  (:Pressed
    (if (Utilities|Enum|NotEqual(Enum) (Variables|Default|GetcurrentMoveMode) "BackViewMode")
      (bind _checkresult (CallFunction|ChangeViewCheck "BackViewMode"))
      (if _checkresult
        (Variables|Default|SetcurrentMoveMode "BackViewMode")
        (Transformation|SetRelativeLocationAndRotation (Variables|Default|GetCameraComponent) "-1620.000000,0.000000,80.000000" "0, 0, 0" false false)
        (bind _asanim_test_character_j_bp (Utilities|Casting|CastToAnimTestCharacter_j_BP (Game|GetPlayerCharacter 0)))
        (Transformation|SetActorRelativeRotation _asanim_test_character_j_bp)
        (Pawn|SetControlRotation (Game|GetPlayerController 0) (Math|Rotator|MakeRotator 0.0 0.0 0.0))))))

(event Input|KeyboardEvents|K
  (params (Key :type Key%20Structure :default "None")))

(fn ConstructionScript)

(fn RollCoolDown
  (bind _output_get (Variables|Default|Setroll%20cooldown (- (Variables|Default|Getroll%20cooldown) 0.1)))
  (if (<= _output_get 0.0)
    (Variables|Default|SetrollCooltime false)
    (Utilities|Time|ClearandInvalidateTimerbyHandle (Variables|Default|GetrcdTH))
    (Variables|Default|Setroll%20cooldown 2.5)
    (else
      (Development|PrintString (Utilities|String|ToString(Float) (Variables|Default|Getroll%20cooldown))))))

(fn ChangeViewCheck
  (params (MoveMode :type EMoveMode%20Enum :default "normal"))
  (bind _self self)
  (bind _self_2 self)
  (bind _self_3 self)
  (bind _self_4 self)
  (bind _returnvalue (Transformation|GetActorLocation _self_2))
  (bind _returnvalue_2 (Transformation|GetActorLocation _self_3))
  (bind _returnvalue_3 (Transformation|GetActorLocation _self))
  (bind _returnvalue_4 (Transformation|GetActorLocation _self_4))
  (bind (_x _y _z) (Math|Vector|BreakVector _returnvalue_2))
  (bind (_x_2 _y_2 _z_2) (Math|Vector|BreakVector _returnvalue_3))
  (bind (_x_3 _y_3 _z_3) (Math|Vector|BreakVector _returnvalue_4))
  (bind (_x_4 _y_4 _z_4) (Math|Vector|BreakVector _returnvalue))
  (switch Utilities|FlowControl|Switch|SwitchonEMoveMode MoveMode
    (:QuarterViewMode
      ;[1 1 1] 쿼터뷰 세팅
      (if (Utilities|Array|IsValidIndex (Variables|Default|GetSideWallArray))
        (CallFunction|SetVisible true (Variables|Default|GetSideWallArray)))
      (if (Utilities|Array|IsValidIndex (Variables|Default|GetBackWallArray))
        (CallFunction|SetVisible true (Variables|Default|GetBackWallArray)))
      (return true))
    (:SideViewMode
      ;[1 1 1] 사이드 뷰 세팅
      (if (Utilities|Array|IsValidIndex (Variables|Default|GetBackWallArray))
        (Development|PrintString "기존 Wall 재생성")
        (else
          (Development|PrintString "일반 사이드 뷰")))
      (bind (_outhit _returnvalue_5) (Collision|CapsuleTraceByChannel _returnvalue (Math|Vector|MakeVector _x_4 (+ _y_4 1e+04) _z_4) 34.0 44.0 "TraceTypeQuery3" false 0 "ForDuration"))
      (if _returnvalue_5
        (if (Components|ComponentHasTag (.HitComponent (Collision|BreakHitResult _outhit)) "Wall")
          (Variables|Default|SetWallComponent1 (.HitComponent (Collision|BreakHitResult _outhit)))
          (else
            (Development|PrintString "물체와 겹칩니다.")
            (return false))))
      (bind (_outhit_2 _returnvalue_6) (Collision|CapsuleTraceByChannel _returnvalue_2 (Math|Vector|MakeVector _x (+ _y -1e+04) _z) 34.0 44.0 "TraceTypeQuery3" false 0 "ForDuration"))
      (if _returnvalue_6
        (if (Components|ComponentHasTag (.HitComponent (Collision|BreakHitResult _outhit_2)) "Wall")
          (Variables|Default|SetWallComponent2 (.HitComponent (Collision|BreakHitResult _outhit_2)))
          (Variables|Default|SetSideWallArray (Utilities|Array|MakeArray (Variables|Default|GetWallComponent1) (Variables|Default|GetWallComponent2)))
          (Development|PrintString "사이드뷰 전환")
          (CallFunction|SetVisible false (Variables|Default|GetSideWallArray))
          (CallFunction|SetVisible true (Variables|Default|GetBackWallArray))
          (return true)
          (else
            (return false)))
        (else
          (return true))))
    (:TopViewMode
      ;[1 1 1] 탑뷰 세팅
      (if (Utilities|Array|IsValidIndex (Variables|Default|GetSideWallArray))
        (CallFunction|SetVisible true (Variables|Default|GetSideWallArray)))
      (if (Utilities|Array|IsValidIndex (Variables|Default|GetBackWallArray))
        (CallFunction|SetVisible false (Variables|Default|GetBackWallArray)))
      (return true))
    (:BackViewMode
      ;[1 1 1] 백뷰 세팅
      (if (Utilities|Array|IsValidIndex (Variables|Default|GetSideWallArray))
        (Development|PrintString "기존 Wall 재생성")
        (else
          (Development|PrintString "일반 백뷰")))
      (bind (_outhit_3 _returnvalue_7) (Collision|CapsuleTraceByChannel _returnvalue_4 (Math|Vector|MakeVector (+ _x_3 1e+04) _y_3 _z_3) 34.0 44.0 "TraceTypeQuery3" false 0 "ForDuration"))
      (if _returnvalue_7
        (if (Components|ComponentHasTag (.HitComponent (Collision|BreakHitResult _outhit_3)) "Wall")
          (Variables|Default|SetWallComponent1 (.HitComponent (Collision|BreakHitResult _outhit_3)))
          (else
            (Development|PrintString "물체와 겹칩니다.")
            (Development|PrintString (Utilities|GetDisplayName (.HitComponent (Collision|BreakHitResult _outhit_3))))
            (return false))))
      (bind (_outhit_4 _returnvalue_8) (Collision|CapsuleTraceByChannel _returnvalue_3 (Math|Vector|MakeVector (+ _x_2 -1e+04) _y_2 _z_2) 34.0 44.0 "TraceTypeQuery3" false 0 "ForDuration"))
      (if _returnvalue_8
        (if (Components|ComponentHasTag (.HitComponent (Collision|BreakHitResult _outhit_4)) "Wall")
          (Variables|Default|SetWallComponent2 (.HitComponent (Collision|BreakHitResult _outhit_4)))
          (Variables|Default|SetBackWallArray (Utilities|Array|MakeArray (Variables|Default|GetWallComponent1) (Variables|Default|GetWallComponent2)))
          (Development|PrintString "백뷰 전환")
          (CallFunction|SetVisible false (Variables|Default|GetBackWallArray))
          (CallFunction|SetVisible true (Variables|Default|GetSideWallArray))
          (return true)
          (else
            (return false)))
        (else
          (return true))))))

(fn SetVisible
  (params (Visible :type Boolean) (Target%20Array :type Array%20of%20Primitive%20Component%20Object%20References))
  (bind _output_get (LocalVariables|SetMyTargetArray Target%20Array))
  (if (Utilities|Array|IsValidIndex _output_get)
    (if Visible
      (for _array_element (LocalVariables|GetMyTargetArray)
        (Rendering|SetVisibility _array_element true false)
        (Collision|SetCollisionEnabled _array_element "QueryAndPhysics"))
      (else
        (for _array_element_2 (LocalVariables|GetMyTargetArray)
          (Rendering|SetVisibility _array_element_2 false false)
          (Collision|SetCollisionEnabled _array_element_2 "NoCollision"))))
    (else
      (Development|PrintString "No array"))))

(fn RemoveWallIndex
  (params (Target%20Array :type Array%20of%20Primitive%20Component%20Object%20References))
  (if (Utilities|Array|IsValidIndex Target%20Array)
    (for _array_element Target%20Array
      (bind _returnvalue (Utilities|Array|RemoveItem Target%20Array _array_element))
      (Development|PrintString (Utilities|String|ToString(Boolean) _returnvalue)))
    (else
      (Development|PrintString "ValidFalse"))))