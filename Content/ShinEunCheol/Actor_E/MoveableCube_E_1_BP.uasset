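; Pushable cube that the player character shoves along X or Y in a game with side and back camera views.
; Overlapping either axis trigger enables cube physics and sets the character's push direction, rotation lock and speed; leaving reverts them.
; Tick polls the player's view flags to toggle per-view blocking colliders.
; Side view also widens the X trigger along Y, shrinking it back when IsDecrease is set.
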(event OnComponentBeginOverlap(XAxis)
  (params (OverlappedComponent :type Primitive%20Component%20Object%20Reference) (OtherActor :type Actor%20Object%20Reference) (OtherComp :type Primitive%20Component%20Object%20Reference) (OtherBodyIndex :type Integer) (bFromSweep :type Boolean) (SweepResult :type Hit%20Result%20Structure%20%28by%20ref%29))
  ;[1 1 1] X 축 밀기 IN
  (bind _asanim_test_character_j_bp (Utilities|Casting|CastToAnimTestCharacter_j_BP OtherActor))
  (Physics|SetSimulatePhysics (Variables|Default|GetCube) true)
  (Variables|/Script/GraduationWork22.AnimTestCharacter_j|SetIsPushing2 _asanim_test_character_j_bp true)
  (if (<= (.x (Transformation|GetActorLocation _asanim_test_character_j_bp)) (.x (Transformation|GetActorLocation self)))
    (Default|PushMode _asanim_test_character_j_bp)
    (else
      (Default|PushMode _asanim_test_character_j_bp 2)))
  (Variables|/Script/Engine.CharacterMovementComponent|SetbOrientRotationToMovement (Variables|/Script/Engine.Character|GetCharacterMovement _asanim_test_character_j_bp) false)
  (Variables|/Script/Engine.CharacterMovementComponent|SetMaxWalkSpeed (Variables|/Script/Engine.Character|GetCharacterMovement _asanim_test_character_j_bp) (Variables|/Script/GraduationWork22.AnimTestCharacter_j|GetpushSpeed _asanim_test_character_j_bp)))

(event OnComponentEndOverlap(XAxis)
  (params (OverlappedComponent :type Primitive%20Component%20Object%20Reference) (OtherActor :type Actor%20Object%20Reference) (OtherComp :type Primitive%20Component%20Object%20Reference) (OtherBodyIndex :type Integer))
  ;[1 1 1] X축 밀기 OUT
  (bind _asanim_test_character_j_bp (Utilities|Casting|CastToAnimTestCharacter_j_BP OtherActor))
  (Physics|SetSimulatePhysics (Variables|Default|GetCube) false)
  (Variables|/Script/GraduationWork22.AnimTestCharacter_j|SetIsPushing2 _asanim_test_character_j_bp false)
  (Variables|/Script/Engine.CharacterMovementComponent|SetbOrientRotationToMovement (Variables|/Script/Engine.Character|GetCharacterMovement _asanim_test_character_j_bp) true)
  (Variables|/Script/Engine.CharacterMovementComponent|SetMaxWalkSpeed (Variables|/Script/Engine.Character|GetCharacterMovement _asanim_test_character_j_bp) (Variables|/Script/GraduationWork22.AnimTestCharacter_j|GetwalkSpeed _asanim_test_character_j_bp)))

(event OnComponentBeginOverlap(YAxis)
  (params (OverlappedComponent :type Primitive%20Component%20Object%20Reference) (OtherActor :type Actor%20Object%20Reference) (OtherComp :type Primitive%20Component%20Object%20Reference) (OtherBodyIndex :type Integer) (bFromSweep :type Boolean) (SweepResult :type Hit%20Result%20Structure%20%28by%20ref%29))
  ;[1 1 1] Y축 밀기 IN
  (bind _asanim_test_character_j_bp (Utilities|Casting|CastToAnimTestCharacter_j_BP OtherActor))
  (Physics|SetSimulatePhysics (Variables|Default|GetCube) true)
  (Variables|/Script/GraduationWork22.AnimTestCharacter_j|SetIsPushing2 _asanim_test_character_j_bp true)
  (if (<= (.y (Transformation|GetActorLocation _asanim_test_character_j_bp)) (.y (Transformation|GetActorLocation self)))
    (Default|PushMode _asanim_test_character_j_bp 1)
    (else
      (Default|PushMode _asanim_test_character_j_bp 3)))
  (Variables|/Script/Engine.CharacterMovementComponent|SetbOrientRotationToMovement (Variables|/Script/Engine.Character|GetCharacterMovement _asanim_test_character_j_bp) false)
  (Variables|/Script/Engine.CharacterMovementComponent|SetMaxWalkSpeed (Variables|/Script/Engine.Character|GetCharacterMovement _asanim_test_character_j_bp) (Variables|/Script/GraduationWork22.AnimTestCharacter_j|GetpushSpeed _asanim_test_character_j_bp)))

(event OnComponentEndOverlap(YAxis)
  (params (OverlappedComponent :type Primitive%20Component%20Object%20Reference) (OtherActor :type Actor%20Object%20Reference) (OtherComp :type Primitive%20Component%20Object%20Reference) (OtherBodyIndex :type Integer))
  ;[1 1 1] Y축 밀기 OUT
  (bind _asanim_test_character_j_bp (Utilities|Casting|CastToAnimTestCharacter_j_BP OtherActor))
  (Physics|SetSimulatePhysics (Variables|Default|GetCube) false)
  (Variables|/Script/GraduationWork22.AnimTestCharacter_j|SetIsPushing2 _asanim_test_character_j_bp false)
  (Variables|/Script/Engine.CharacterMovementComponent|SetbOrientRotationToMovement (Variables|/Script/Engine.Character|GetCharacterMovement _asanim_test_character_j_bp) true)
  (Variables|/Script/Engine.CharacterMovementComponent|SetMaxWalkSpeed (Variables|/Script/Engine.Character|GetCharacterMovement _asanim_test_character_j_bp) (Variables|/Script/GraduationWork22.AnimTestCharacter_j|GetwalkSpeed _asanim_test_character_j_bp)))

(event EventBeginPlay
  (bind _asanim_test_character_j_bp (Utilities|Casting|CastToAnimTestCharacter_j_BP (Game|GetPlayerCharacter 0)))
  (Variables|Default|SetMyCharacter _asanim_test_character_j_bp)
  (Collision|SetCollisionEnabled (Variables|Default|GetSideViewCube) "NoCollision")
  (Collision|SetCollisionEnabled (Variables|Default|GetBackViewCube) "NoCollision"))

(event EventTick
  (params (DeltaSeconds :type Float%20%28single-precision%29))
  (bind _x_axis (Variables|Default|GetX%20Axis))
  (bind _relativescale3d (Variables|/Script/Engine.SceneComponent|GetRelativeScale3D _x_axis))
  (bind _relativelocation (Variables|/Script/Engine.SceneComponent|GetRelativeLocation _x_axis))
  (Utilities|FlowControl|Sequence
    (:then_0
      (bind _asanim_test_character_j_bp (Utilities|Casting|CastToAnimTestCharacter_j_BP (Game|GetPlayerCharacter 0)))
      (if (Variables|/Game/ShimJaeChun/Character_j/AnimTestCharacter_j_BP.AnimTestCharacter_j_BP_C|GetisSideView _asanim_test_character_j_bp)
        (CallFunction|SidePlayerBlock)
        (else
          (CallFunction|SidePlayerUnBlock)))
      (if (Variables|/Game/ShimJaeChun/Character_j/AnimTestCharacter_j_BP.AnimTestCharacter_j_BP_C|GetisBackView _asanim_test_character_j_bp)
        (CallFunction|BackPlayerBlock)
        (else
          (CallFunction|BackPlayerUnBlock))))
    (:then_1
      (bind _asanim_test_character_j_bp_2 (Utilities|Casting|CastToAnimTestCharacter_j_BP (Game|GetPlayerCharacter 0)))
      (if (Variables|/Game/ShimJaeChun/Character_j/AnimTestCharacter_j_BP.AnimTestCharacter_j_BP_C|GetisSideView _asanim_test_character_j_bp_2)
        (Transformation|SetRelativeTransform _x_axis (Math|Transform|MakeTransform _relativelocation "0, 0, 0" (Math|Vector|MakeVector (.x _relativescale3d) 15.0 (.z _relativescale3d))) false false)
        (elif (Variables|/Game/ShimJaeChun/Character_j/AnimTestCharacter_j_BP.AnimTestCharacter_j_BP_C|GetIsDecrease _asanim_test_character_j_bp_2)
          (Transformation|SetRelativeTransform _x_axis (Math|Transform|MakeTransform _relativelocation "0, 0, 0" (Math|Vector|MakeVector (.x _relativescale3d) 0.627085 (.z _relativescale3d))) false false))))))

(event Collision|EventActorBeginOverlap
  (params (OtherActor :type Actor%20Object%20Reference)))

(fn ConstructionScript)

(fn SidePlayerBlock
  (Collision|SetCollisionResponsetoChannel (Variables|Default|GetSideViewCube) "ECC_Pawn" "ECR_Block")
  (Collision|SetCollisionEnabled (Variables|Default|GetSideViewCube) "QueryAndPhysics"))

(fn SidePlayerUnBlock
  (Collision|SetCollisionResponsetoChannel (Variables|Default|GetSideViewCube) "ECC_Pawn" "ECR_Ignore")
  (Collision|SetCollisionEnabled (Variables|Default|GetSideViewCube) "NoCollision"))

(fn BackPlayerBlock
  (Collision|SetCollisionResponsetoChannel (Variables|Default|GetBackViewCube) "ECC_Pawn" "ECR_Block")
  (Collision|SetCollisionEnabled (Variables|Default|GetBackViewCube) "QueryAndPhysics"))

(fn BackPlayerUnBlock
  (Collision|SetCollisionResponsetoChannel (Variables|Default|GetBackViewCube) "ECC_Pawn" "ECR_Block")
  (Collision|SetCollisionEnabled (Variables|Default|GetBackViewCube) "NoCollision"))