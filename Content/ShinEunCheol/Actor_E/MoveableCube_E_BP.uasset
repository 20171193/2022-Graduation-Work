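; A pushable cube actor that the AnimTestCharacter_j_BP character can shove when it enters the XAxis or YAxis trigger volume.
; Entering either trigger enables physics on the cube and puts the character in pushing mode with push speed and no orient-to-movement; leaving reverses this.
; Every tick, the player's IsSideView and IsBackView flags toggle SideViewCube and BackViewCube collision, creating view-dependent blockers.
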(event OnComponentBeginOverlap(XAxis)
  (params (OverlappedComponent :type Primitive%20Component%20Object%20Reference) (OtherActor :type Actor%20Object%20Reference) (OtherComp :type Primitive%20Component%20Object%20Reference) (OtherBodyIndex :type Integer) (bFromSweep :type Boolean) (SweepResult :type Hit%20Result%20Structure%20%28by%20ref%29))
  (bind _asanim_test_character_j_bp (Utilities|Casting|CastToAnimTestCharacter_j_BP OtherActor))
  (Physics|SetSimulatePhysics (Variables|Default|GetCube) true)
  (Variables|/Script/GraduationWork22.AnimTestCharacter_j|SetIsPushing2 _asanim_test_character_j_bp true)
  (Variables|/Script/Engine.CharacterMovementComponent|SetbOrientRotationToMovement (Variables|/Script/Engine.Character|GetCharacterMovement _asanim_test_character_j_bp) false)
  (Variables|/Script/Engine.CharacterMovementComponent|SetMaxWalkSpeed (Variables|/Script/Engine.Character|GetCharacterMovement _asanim_test_character_j_bp) (Variables|/Script/GraduationWork22.AnimTestCharacter_j|GetpushSpeed _asanim_test_character_j_bp)))

(event OnComponentEndOverlap(XAxis)
  (params (OverlappedComponent :type Primitive%20Component%20Object%20Reference) (OtherActor :type Actor%20Object%20Reference) (OtherComp :type Primitive%20Component%20Object%20Reference) (OtherBodyIndex :type Integer))
  (bind _asanim_test_character_j_bp (Utilities|Casting|CastToAnimTestCharacter_j_BP OtherActor))
  (Physics|SetSimulatePhysics (Variables|Default|GetCube) false)
  (Variables|/Script/GraduationWork22.AnimTestCharacter_j|SetIsPushing2 _asanim_test_character_j_bp false)
  (Variables|/Script/Engine.CharacterMovementComponent|SetbOrientRotationToMovement (Variables|/Script/Engine.Character|GetCharacterMovement _asanim_test_character_j_bp) true)
  (Variables|/Script/Engine.CharacterMovementComponent|SetMaxWalkSpeed (Variables|/Script/Engine.Character|GetCharacterMovement _asanim_test_character_j_bp) (Variables|/Script/GraduationWork22.AnimTestCharacter_j|GetwalkSpeed _asanim_test_character_j_bp)))

(event OnComponentBeginOverlap(YAxis)
  (params (OverlappedComponent :type Primitive%20Component%20Object%20Reference) (OtherActor :type Actor%20Object%20Reference) (OtherComp :type Primitive%20Component%20Object%20Reference) (OtherBodyIndex :type Integer) (bFromSweep :type Boolean) (SweepResult :type Hit%20Result%20Structure%20%28by%20ref%29))
  (bind _asanim_test_character_j_bp (Utilities|Casting|CastToAnimTestCharacter_j_BP OtherActor))
  (Physics|SetSimulatePhysics (Variables|Default|GetCube) true)
  (Variables|/Script/GraduationWork22.AnimTestCharacter_j|SetIsPushing2 _asanim_test_character_j_bp true)
  (Variables|/Script/Engine.CharacterMovementComponent|SetbOrientRotationToMovement (Variables|/Script/Engine.Character|GetCharacterMovement _asanim_test_character_j_bp) false)
  (Variables|/Script/Engine.CharacterMovementComponent|SetMaxWalkSpeed (Variables|/Script/Engine.Character|GetCharacterMovement _asanim_test_character_j_bp) (Variables|/Script/GraduationWork22.AnimTestCharacter_j|GetpushSpeed _asanim_test_character_j_bp)))

(event OnComponentEndOverlap(YAxis)
  (params (OverlappedComponent :type Primitive%20Component%20Object%20Reference) (OtherActor :type Actor%20Object%20Reference) (OtherComp :type Primitive%20Component%20Object%20Reference) (OtherBodyIndex :type Integer))
  (bind _asanim_test_character_j_bp (Utilities|Casting|CastToAnimTestCharacter_j_BP OtherActor))
  (Physics|SetSimulatePhysics (Variables|Default|GetCube) false)
  (Variables|/Script/GraduationWork22.AnimTestCharacter_j|SetIsPushing2 _asanim_test_character_j_bp false)
  (Variables|/Script/Engine.CharacterMovementComponent|SetbOrientRotationToMovement (Variables|/Script/Engine.Character|GetCharacterMovement _asanim_test_character_j_bp) true)
  (Variables|/Script/Engine.CharacterMovementComponent|SetMaxWalkSpeed (Variables|/Script/Engine.Character|GetCharacterMovement _asanim_test_character_j_bp) (Variables|/Script/GraduationWork22.AnimTestCharacter_j|GetwalkSpeed _asanim_test_character_j_bp)))

(event EventTick
  (params (DeltaSeconds :type Float%20%28single-precision%29))
  (bind _asanim_test_character_j_bp (Utilities|Casting|CastToAnimTestCharacter_j_BP (Game|GetPlayerCharacter 0)))
  (if (Variables|/Game/ShimJaeChun/Character_j/AnimTestCharacter_j_BP.AnimTestCharacter_j_BP_C|GetisSideView _asanim_test_character_j_bp)
    (CallFunction|SidePlayerBlock)
    (else
      (CallFunction|SidePlayerUnBlock)))
  (if (Variables|/Game/ShimJaeChun/Character_j/AnimTestCharacter_j_BP.AnimTestCharacter_j_BP_C|GetisBackView _asanim_test_character_j_bp)
    (CallFunction|BackPlayerBlock)
    (else
      (CallFunction|BackPlayerUnBlock))))

(event EventBeginPlay
  (Collision|SetCollisionEnabled (Variables|Default|GetSideViewCube) "NoCollision")
  (Collision|SetCollisionEnabled (Variables|Default|GetBackViewCube) "NoCollision"))

(event Collision|EventActorBeginOverlap
  (params (OtherActor :type Actor%20Object%20Reference)))

(fn ConstructionScript)

(fn SidePlayerBlock
  (Collision|SetCollisionResponsetoChannel (Variables|Default|GetSideViewCube) "ECC_Pawn" "ECR_Block")
  (Collision|SetCollisionEnabled (Variables|Default|GetSideViewCube) "QueryAndPhysics"))

(fn SidePlayerUnBlock
  (Collision|SetCollisionResponsetoChannel (Variables|Default|GetSideViewCube) "ECC_Pawn" "ECR_Ignore")
  (Collision|SetCollisionEnabled (Variables|Default|GetSideViewCube) "NoCollision"))

(fn BackPlayerBlock
  (Collision|SetCollisionResponsetoChannel (Variables|Default|GetBackViewCube) "ECC_Pawn" "ECR_Block")
  (Collision|SetCollisionEnabled (Variables|Default|GetBackViewCube) "QueryAndPhysics"))

(fn BackPlayerUnBlock
  (Collision|SetCollisionResponsetoChannel (Variables|Default|GetBackViewCube) "ECC_Pawn" "ECR_Block")
  (Collision|SetCollisionEnabled (Variables|Default|GetBackViewCube) "NoCollision"))