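; Test player character with switchable camera modes (quarter, top, side, back), ladder climbing and a dodge roll.
; View keys reposition the camera and reset character and control rotation; F toggles flying and snaps to a nearby ladder by its yaw.
; Damage plays hit reactions with knockback chosen by the causer's yaw, or death and unpossess, though HP currently subtracts zero.
; Roll briefly flies during its montage, gated by a timer-driven cooldown.
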(event Collision|EventActorBeginOverlap
  (params (OtherActor :type Actor%20Object%20Reference)))

(event EventBeginPlay
  ;[1 1 1] 플레이어 시작 세팅 - 쿼터뷰
  (Variables|Default|SetcurrentMoveMode "QuarterViewMode")
  (Transformation|SetRelativeLocationAndRotation (Variables|Default|GetCameraComponent) "-535.000000,7.500000,1135.000000" "-50.000000,0.000000,0.000000" false false)
  (bind _asanim_test_character_j_bp (Utilities|Casting|CastToAnimTestCharacter_j_BP (Game|GetPlayerCharacter 0)))
  (Transformation|SetActorRelativeRotation _asanim_test_character_j_bp "0,-50.000000,0.000000")
  (Pawn|SetControlRotation (Game|GetPlayerController 0) (Math|Rotator|MakeRotator 0.0 0.0 -5e+01)))

(event Game|Damage|EventAnyDamage
  (params (Damage :type Float%20%28single-precision%29) (DamageType :type Damage%20Type%20Object%20Reference) (InstigatedBy :type Controller%20Object%20Reference) (DamageCauser :type Actor%20Object%20Reference))
  ;[1 1 1] 데미지처리
  (if (<= (- (Variables|Default|GetplayerHp) (Math|Float|Truncate Damage)) 0)
    ;[1 1 1] Death처리
    (Animation|PlayAnimMontage "/Game/ShimJaeChun/Anim_j/StandingDeath_AMG_j.StandingDeath_AMG_j" 1.0 "None")
    (Utilities|FlowControl|Delay 2.0)
    (Pawn|UnPossess (Pawn|GetController (Game|GetPlayerCharacter 0)))
    (else
      ;[1 1 1] 피격 처리
      (if (Utilities|IsValid DamageCauser)
        (bind _output_get (Variables|Default|SetdamageActorRotZ (.yaw (Transformation|GetActorRotation DamageCauser))))
        (Development|PrintString (Utilities|String|ToString(Float) _output_get))
        (if (and (<= (Variables|Default|GetdamageActorRotZ) 1e+01) (> (Variables|Default|GetdamageActorRotZ) -1e+01))
          (Development|PrintString "0도")
          (Character|LaunchCharacter self (Math|Vector|MakeVector 0.0 1e+03 5e+01) true false)
          (Variables|Default|SetplayerHp (Math|Float|Truncate (- (Math|Conversions|ToFloat(Integer) (Variables|Default|GetplayerHp)) 0.0)) :!label _label)
          (Animation|PlayAnimMontage "/Game/ShimJaeChun/Anim_j/HitReaction_AM.HitReaction_AM" 1.0 "None")
          (elif (or (and (<= (Variables|Default|GetdamageActorRotZ) 1e+02) (> (Variables|Default|GetdamageActorRotZ) 8e+01)) (and (<= (Variables|Default|GetdamageActorRotZ) -2.6e+02) (> (Variables|Default|GetdamageActorRotZ) -2.8e+02)))
            (Development|PrintString "90, -270도")
            (Character|LaunchCharacter self (Math|Vector|MakeVector -1e+03 0.0 5e+01) true true)
            (goto _label)
            (elif (or (and (<= (Variables|Default|GetdamageActorRotZ) 1.9e+02) (> (Variables|Default|GetdamageActorRotZ) 1.7e+02)) (and (<= (Variables|Default|GetdamageActorRotZ) -1.7e+02) (> (Variables|Default|GetdamageActorRotZ) -1.9e+02)))
              (Development|PrintString "180, -180도")
              (Character|LaunchCharacter self (Math|Vector|MakeVector 0.0 -1e+03 5e+01) true false)
              (goto _label)
              (elif (or (and (<= (Variables|Default|GetdamageActorRotZ) 2.8e+02) (> (Variables|Default|GetdamageActorRotZ) 2.6e+02)) (and (<= (Variables|Default|GetdamageActorRotZ) -8e+01) (> (Variables|Default|GetdamageActorRotZ) -1e+02)))
                (Development|PrintString "270, -90도")
                (Character|LaunchCharacter self (Math|Vector|MakeVector 1e+03 0.0 5e+01) true false)
                (goto _label)))))))))

(event Input|ActionEvents|InputActionRoll
  (params (Key :type Key%20Structure :default "None"))
  (bind _charactermovement (Variables|Character|GetCharacterMovement))
  (bind _charactermovement_2 (Variables|Character|GetCharacterMovement))
  ;[1 1 1] 구르기
  (:Pressed
    (if (Variables|Default|GetrollAble)
      (if (Variables|Default|GetrollCooltime)
        (Development|PrintString "Not yet Roll" :!label _label)
        (else
          (Variables|Default|SetrollCooltime true)
          (bind _returnvalue (Utilities|Time|SetTimerbyFunctionName self "Roll Cool Down" 0.1 true))
          (Variables|Default|SetrcdTH _returnvalue)
          (Pawn|Components|CharacterMovement|SetMovementMode _charactermovement_2 "MOVE_Flying" 0)
          (Variables|/Script/Engine.CharacterMovementComponent|SetMaxFlySpeed _charactermovement_2 8e+02)
          (bind _returnvalue_2 (Animation|PlayAnimMontage "/Game/ShimJaeChun/Anim_j/Rolling_AMG_j.Rolling_AMG_j" 1.5 "None"))
          (Utilities|FlowControl|Delay (- _returnvalue_2 0.5))
          (Pawn|Components|CharacterMovement|SetMovementMode _charactermovement "MOVE_Walking" 0)
          (Variables|/Script/Engine.CharacterMovementComponent|SetMaxFlySpeed _charactermovement 6e+02)))
      (else
        (goto _label)))))

(event Input|KeyboardEvents|F
  (params (Key :type Key%20Structure :default "None"))
  (bind _returnvalue (Game|GetPlayerCharacter 0))
  ;[1 1 1] 사다리 타기
  (:Pressed
    (if (Variables|Default|Getclimbable2)
      (if (Variables|Default|GetIsLadder2)
        (Utilities|FlowControl|Sequence
          (:then_0
            (goto _label Reset))
          (:then_1
            ;[1 1 1] 사다리 추락
            (Transformation|SetActorRelativeLocation (+ (Transformation|GetActorLocation _returnvalue) (* (Transformation|GetActorForwardVector _returnvalue) -5e+01)))
            (Pawn|Components|CharacterMovement|SetMovementMode (Variables|Character|GetCharacterMovement) "MOVE_Falling" 0)))
        (else
          (Pawn|Components|CharacterMovement|SetMovementMode (Variables|Character|GetCharacterMovement) "MOVE_Flying" 0)
          (Variables|Default|SetIsLadder2 true)
          (Utilities|FlowControl|Sequence
            (:then_0
              (Utilities|FlowControl|DoOnce false :!label _label
                (:Completed
                  (bind _outactors (Actor|GetAllActorsOfClass "/Game/ShimJaeChun/Actor_j/Ledder_j_BP.Ledder_j_BP_C"))
                  (bind (_array_element _array_index) (Utilities|Array|ForEachLoopwithBreak _outactors :!label _label_2)
                    (:LoopBody
                      (bind _asanim_test_character_j_bp (Utilities|Casting|CastToAnimTestCharacter_j_BP (Game|GetPlayerCharacter 0)))
                      (if (<= (Transformation|GetDistanceTo _array_element) 1.8e+02)
                        (Utilities|FlowControl|Sequence
                          (:then_0
                            (Variables|Default|SetLadder%20Index _array_index)
                            (Utilities|FlowControl|Delay 0.1)
                            (Transformation|SetActorRotation (Math|Rotator|MakeRotator (.roll (Transformation|GetActorRotation _asanim_test_character_j_bp)) (.pitch (Transformation|GetActorRotation _asanim_test_character_j_bp)) (+ (.yaw (Transformation|GetActorRotation (Variables|Default|GetLadder%20BP%20ref))) -9e+01)))
                            ;[1 1 1] -> 사다리
                            (Variables|Default|SetPlayer%20Z%20Location (.z (Transformation|GetActorLocation _asanim_test_character_j_bp)))
                            (if (and (<= (.yaw (Transformation|GetActorRotation (Variables|Default|GetLadder%20BP%20ref))) 185.0) (> (.yaw (Transformation|GetActorRotation (Variables|Default|GetLadder%20BP%20ref))) 175.0))
                              (Development|PrintString "->")
                              (Transformation|SetActorLocation (Math|Vector|MakeVector (.x (Transformation|GetActorLocation (Variables|Default|GetLadder%20BP%20ref))) (+ (.y (Transformation|GetActorLocation (Variables|Default|GetLadder%20BP%20ref))) 4e+01) (.z (Transformation|GetActorLocation _asanim_test_character_j_bp))) false false)
                              (else
                                ;[1 1 1] ^ 사다리
                                (if (and (<= (.yaw (Transformation|GetActorRotation (Variables|Default|GetLadder%20BP%20ref))) 95.0) (> (.yaw (Transformation|GetActorRotation (Variables|Default|GetLadder%20BP%20ref))) 85.0))
                                  (Development|PrintString "^")
                                  (Transformation|SetActorLocation (Math|Vector|MakeVector (- (.x (Transformation|GetActorLocation (Variables|Default|GetLadder%20BP%20ref))) 4e+01) (.y (Transformation|GetActorLocation (Variables|Default|GetLadder%20BP%20ref))) (Variables|Default|GetPlayer%20Z%20Location)) false false)
                                  (else
                                    ;[1 1 1] V 사다리
                                    (if (and (<= (.yaw (Transformation|GetActorRotation (Variables|Default|GetLadder%20BP%20ref))) 275.0) (> (.yaw (Transformation|GetActorRotation (Variables|Default|GetLadder%20BP%20ref))) 265.0))
                                      (Development|PrintString "V")
                                      (Transformation|SetActorLocation (Math|Vector|MakeVector (+ (.x (Transformation|GetActorLocation (Variables|Default|GetLadder%20BP%20ref))) 4e+01) (.y (Transformation|GetActorLocation (Variables|Default|GetLadder%20BP%20ref))) (Variables|Default|GetPlayer%20Z%20Location)) false false)
                                      (else
                                        ;[1 1 1] <- 사다리
                                        (if (and (<= (.yaw (Transformation|GetActorRotation (Variables|Default|GetLadder%20BP%20ref))) 5.0) (> (.yaw (Transformation|GetActorRotation (Variables|Default|GetLadder%20BP%20ref))) -5.0))
                                          (Development|PrintString "<-")
                                          (Transformation|SetActorLocation (Math|Vector|MakeVector (.x (Transformation|GetActorLocation (Variables|Default|GetLadder%20BP%20ref))) (+ (.y (Transformation|GetActorLocation (Variables|Default|GetLadder%20BP%20ref))) 4e+01) (Variables|Default|GetPlayer%20Z%20Location)) false false)))))))))
                          (:then_1
                            (goto _label_2 Break))
                          (:then_2
                            (Variables|Default|SetLadder%20BP%20ref (Utilities|Array|Get(acopy) _outactors (Variables|Default|GetLadder%20Index)))))))))))))))))

(event Input|KeyboardEvents|A
  (params (Key :type Key%20Structure :default "None"))
  ;[1 1 1] 사이드 뷰모드 세팅
  (:Pressed
    (Variables|Default|SetSideViewCheck true)
    (Variables|Default|SetcurrentMoveMode "SideViewMode")
    (Transformation|SetRelativeLocationAndRotation (Variables|Default|GetCameraComponent) "0.000000,-600.000000,100.000000" "0.000000,90.000000,0.000000" false false)
    (bind _asanim_test_character_j_bp (Utilities|Casting|CastToAnimTestCharacter_j_BP (Game|GetPlayerCharacter 0)))
    (Transformation|SetActorRelativeRotation _asanim_test_character_j_bp)
    (Pawn|SetControlRotation (Game|GetPlayerController 0) (Math|Rotator|MakeRotator 0.0 0.0 0.0))))

(event Input|KeyboardEvents|W
  (params (Key :type Key%20Structure :default "None"))
  ;[1 1 1] 탑 뷰모드 세팅
  (:Pressed
    (Variables|Default|SetcurrentMoveMode "TopViewMode")
    (Transformation|SetRelativeLocationAndRotation (Variables|Default|GetCameraComponent) "300.000000,0.000000,1000.000000" "-90.000000,0.000000,0.000000" false false)
    (bind _asanim_test_character_j_bp (Utilities|Casting|CastToAnimTestCharacter_j_BP (Game|GetPlayerCharacter 0)))
    (Transformation|SetActorRelativeRotation _asanim_test_character_j_bp)
    (Pawn|SetControlRotation (Game|GetPlayerController 0) (Math|Rotator|MakeRotator 0.0 0.0 0.0))))

(event Input|KeyboardEvents|D
  (params (Key :type Key%20Structure :default "None"))
  ;[1 1 1] 쿼터 뷰모드 세팅
  (:Pressed
    (Variables|Default|SetSideViewCheck false)
    (Variables|Default|SetcurrentMoveMode "QuarterViewMode")
    (Transformation|SetRelativeLocationAndRotation (Variables|Default|GetCameraComponent) "-535.000000,7.500000,1135.000000" "-50.000000,0.000000,0.000000" false false)
    (bind _asanim_test_character_j_bp (Utilities|Casting|CastToAnimTestCharacter_j_BP (Game|GetPlayerCharacter 0)))
    (Transformation|SetActorRelativeRotation _asanim_test_character_j_bp "0,-50.000000,0.000000")
    (Pawn|SetControlRotation (Game|GetPlayerController 0) (Math|Rotator|MakeRotator 0.0 0.0 -5e+01))))

(event Input|KeyboardEvents|S
  (params (Key :type Key%20Structure :default "None"))
  ;[1 1 1] 백 뷰모드 세팅
  (:Pressed
    (Variables|Default|SetcurrentMoveMode "BackViewMode")
    (Transformation|SetRelativeLocationAndRotation (Variables|Default|GetCameraComponent) "-1620.000000,0.000000,80.000000" "0, 0, 0" false false)
    (bind _asanim_test_character_j_bp (Utilities|Casting|CastToAnimTestCharacter_j_BP (Game|GetPlayerCharacter 0)))
    (Transformation|SetActorRelativeRotation _asanim_test_character_j_bp)
    (Pawn|SetControlRotation (Game|GetPlayerController 0) (Math|Rotator|MakeRotator 0.0 0.0 0.0))))

(event Input|KeyboardEvents|K
  (params (Key :type Key%20Structure :default "None"))
  (:Pressed
    (Character|LaunchCharacter self "1000.000000, 0,50.000000" false false)))

(fn ConstructionScript)

(fn RollCoolDown
  (bind _output_get (Variables|Default|Setroll%20cooldown (- (Variables|Default|Getroll%20cooldown) 0.1)))
  (if (<= _output_get 0.0)
    (Variables|Default|SetrollCooltime false)
    (Utilities|Time|ClearandInvalidateTimerbyHandle (Variables|Default|GetrcdTH))
    (Variables|Default|Setroll%20cooldown 2.5)
    (else
      (Development|PrintString (Utilities|String|ToString(Float) (Variables|Default|Getroll%20cooldown))))))