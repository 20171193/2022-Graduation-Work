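; Test character Blueprint for ladder climbing and switching between top, side, quarter and back camera views.
; F, when Climbable, sets flying mode, then snaps the player, cast to AnimTestCharacter_j_BP, beside the first Ledder_j_BP found, using yaw-range offsets that skip negative yaws.
; W, A, D and S set the move mode and hard-coded camera transforms, with varying rotation resets; back view is marked unfinished.
; A roll-montage chain is unconnected.
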(event EventBeginPlay)

(event Collision|EventActorBeginOverlap
  (params (OtherActor :type Actor%20Object%20Reference)))

(event Input|ActionEvents|InputActionActRoll
  (params (Key :type Key%20Structure :default "None")))

(event Input|KeyboardEvents|F
  (params (Key :type Key%20Structure :default "None"))
  (:Pressed
    (if (Variables|Default|Getclimbable)
      (Pawn|Components|CharacterMovement|SetMovementMode (Variables|Character|GetCharacterMovement) "MOVE_Flying" 0)
      (Variables|Default|SetisLadder true)
      (bind _outactors (Actor|GetAllActorsOfClass "/Game/ShimJaeChun/Actor_j/Ledder_j_BP.Ledder_j_BP_C"))
      (bind _asanim_test_character_j_bp (Utilities|Casting|CastToAnimTestCharacter_j_BP (Game|GetPlayerCharacter 0)))
      (if (== (.yaw (Transformation|GetActorRotation (Utilities|Array|Get(acopy) _outactors))) 0.0)
        (Transformation|SetActorRotation _asanim_test_character_j_bp (Math|Rotator|MakeRotator (.roll (Transformation|GetActorRotation _asanim_test_character_j_bp)) (.pitch (Transformation|GetActorRotation _asanim_test_character_j_bp)) (- (.yaw (Transformation|GetActorRotation (Utilities|Array|Get(acopy) _outactors))) 9e+01)))
        (Transformation|SetActorLocation _asanim_test_character_j_bp (Math|Vector|MakeVector (.x (Transformation|GetActorLocation (Utilities|Array|Get(acopy) _outactors))) (+ (.y (Transformation|GetActorLocation (Utilities|Array|Get(acopy) _outactors))) 3e+01) (.z (Transformation|GetActorLocation _asanim_test_character_j_bp))) false false)
        (Variables|/Script/Engine.MovementComponent|SetVelocity (Variables|/Script/Engine.Character|GetCharacterMovement _asanim_test_character_j_bp) "0, 0, 0" :!label _label)
        (elif (and (> (.yaw (Transformation|GetActorRotation (Utilities|Array|Get(acopy) _outactors))) 0.0) (<= (.yaw (Transformation|GetActorRotation (Utilities|Array|Get(acopy) _outactors))) 9e+01))
          (Transformation|SetActorRotation _asanim_test_character_j_bp (Math|Rotator|MakeRotator (.roll (Transformation|GetActorRotation _asanim_test_character_j_bp)) (.pitch (Transformation|GetActorRotation _asanim_test_character_j_bp)) (- (.yaw (Transformation|GetActorRotation (Utilities|Array|Get(acopy) _outactors))) 9e+01)))
          (Transformation|SetActorLocation _asanim_test_character_j_bp (Math|Vector|MakeVector (- (.x (Transformation|GetActorLocation (Utilities|Array|Get(acopy) _outactors))) 3e+01) (.y (Transformation|GetActorLocation (Utilities|Array|Get(acopy) _outactors))) (.z (Transformation|GetActorLocation _asanim_test_character_j_bp))) false false)
          (goto _label)
          (elif (and (> (.yaw (Transformation|GetActorRotation (Utilities|Array|Get(acopy) _outactors))) 9e+01) (<= (.yaw (Transformation|GetActorRotation (Utilities|Array|Get(acopy) _outactors))) 1.8e+02))
            (Transformation|SetActorRotation _asanim_test_character_j_bp (Math|Rotator|MakeRotator (.roll (Transformation|GetActorRotation _asanim_test_character_j_bp)) (.pitch (Transformation|GetActorRotation _asanim_test_character_j_bp)) (- (.yaw (Transformation|GetActorRotation (Utilities|Array|Get(acopy) _outactors))) 9e+01)))
            (Transformation|SetActorLocation _asanim_test_character_j_bp (Math|Vector|MakeVector (.x (Transformation|GetActorLocation (Utilities|Array|Get(acopy) _outactors))) (- (.y (Transformation|GetActorLocation (Utilities|Array|Get(acopy) _outactors))) 3e+01) (.z (Transformation|GetActorLocation _asanim_test_character_j_bp))) false false)
            (goto _label)
            (elif (and (> (.yaw (Transformation|GetActorRotation (Utilities|Array|Get(acopy) _outactors))) 1.8e+02) (<= (.yaw (Transformation|GetActorRotation (Utilities|Array|Get(acopy) _outactors))) 2.7e+02))
              (Transformation|SetActorRotation _asanim_test_character_j_bp (Math|Rotator|MakeRotator (.roll (Transformation|GetActorRotation _asanim_test_character_j_bp)) (.pitch (Transformation|GetActorRotation _asanim_test_character_j_bp)) (- (.yaw (Transformation|GetActorRotation (Utilities|Array|Get(acopy) _outactors))) 9e+01)))
              (Transformation|SetActorLocation _asanim_test_character_j_bp (Math|Vector|MakeVector (+ (.x (Transformation|GetActorLocation (Utilities|Array|Get(acopy) _outactors))) 3e+01) (.y (Transformation|GetActorLocation (Utilities|Array|Get(acopy) _outactors))) (.z (Transformation|GetActorLocation _asanim_test_character_j_bp))) false false)
              (goto _label))))))))

(event Input|KeyboardEvents|A
  (params (Key :type Key%20Structure :default "None"))
  ;[1 1 1] 사이드 뷰
  (:Pressed
    (Variables|Default|SetcurrentMoveMode "SideViewMode")
    (Pawn|SetControlRotation (Game|GetPlayerController 0) (Math|Rotator|MakeRotator 0.0 0.0 0.0))
    (Transformation|SetRelativeLocationAndRotation (Variables|Default|GetCameraComponent) "305.000000,-2280.000000,100.000000" "0.000000,90.000000, 0" false false)))

(event Input|KeyboardEvents|W
  (params (Key :type Key%20Structure :default "None"))
  ;[1 1 1] 탑뷰
  (:Pressed
    (Variables|Default|SetcurrentMoveMode "TopViewMode")
    (Pawn|SetControlRotation (Game|GetPlayerController 0) (Math|Rotator|MakeRotator 0.0 0.0 0.0))
    (Transformation|SetActorRotation "0, 0, 0")
    (Transformation|SetRelativeLocationAndRotation (Variables|Default|GetCameraComponent) "300.000000,0.000000,1000.000000" "270.000000,0.000000,0.000000" false false)))

(event Input|KeyboardEvents|D
  (params (Key :type Key%20Structure :default "None"))
  ;[1 1 1] 쿼터뷰
  (:Pressed
    (Variables|Default|SetcurrentMoveMode "QuarterViewMode")
    (Pawn|SetControlRotation (Game|GetPlayerController 0) (Math|Rotator|MakeRotator 0.0 0.0 -5e+01))
    (Transformation|SetActorRelativeRotation "0,-50.000000,0.000000")
    (Transformation|SetRelativeLocationAndRotation (Variables|Default|GetCameraComponent) "-534.000000,7.600000,1137.000000" "-50.000000,0.000000,0.000000" false false)))

(event Input|KeyboardEvents|S
  (params (Key :type Key%20Structure :default "None"))
  ;[1 1 1] 백뷰 (미설정)
  (:Pressed
    (Variables|Default|SetcurrentMoveMode "BackViewMode")
    (Transformation|SetActorRotation "0, 0, 0")
    (Transformation|SetRelativeLocationAndRotation (Variables|Default|GetCameraComponent) "-1620.000000,0.000000,80.000000" "360.000000,0.000000,0.000000" false false)))

(fn ConstructionScript)